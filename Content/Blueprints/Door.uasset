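; Door Blueprint that raises its mesh once enough linked switches are active.
; Activate and Deactivate events adjust a switch count, and reaching SwitchRequirement plays a timeline that offsets the mesh's world Z from its location stored at BeginPlay.
; Dropping below the requirement reverses the timeline, unless StayOpen keeps the door open.
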(event `self.ReceiveBeginPlay`
  (set `self.InitialDoorLocation` (`SceneComponent.K2_GetComponentLocation` (`self.DoorMesh`))))

(event `/Game/Blueprints/SwitchInterface.Activate`
  (`/Engine/EditorBlueprintResources/StandardMacros.IncrementInt` (`self.SwitchesActivated`)
    (:`  `
      (if (>= (`self.SwitchesActivated`) (`self.SwitchRequirement`))
        (bind (_direction _elevation) (`Timeline|DoorTimeline` :!label _label)
          (:`Update`
            (`SceneComponent.K2_SetWorldLocation` (`self.DoorMesh`) (`KismetMathLibrary.MakeVector` (.x (`self.InitialDoorLocation`)) (.y (`self.InitialDoorLocation`)) (+ _elevation (.z (`self.InitialDoorLocation`)))) false false)))))))

(event `/Game/Blueprints/SwitchInterface.Deactivate`
  (`/Engine/EditorBlueprintResources/StandardMacros.DecrementInt` (`self.SwitchesActivated`)
    (:`  `
      (if (< (`self.SwitchesActivated`) (`self.SwitchRequirement`))
        (if (not (`self.StayOpen`))
          (goto _label :!via `Reverse`))))))

(fn `UserConstructionScript`)